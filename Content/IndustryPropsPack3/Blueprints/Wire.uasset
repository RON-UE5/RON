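; Spline-driven wire prop actor that builds an adjustable wire along its Spline component.
; The construction script loops over each segment between spline points and calls Wire, which adds a spline mesh component fitted to both points' local locations and tangents.
; WireSize scales the cross-section at both ends.
; Each segment gets its own dynamic material instance, fed by the Color, Specular and Roughness variables.
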(fn ConstructionScript
  (for _index (range 0 (- (Spline|GetNumberOfSplinePoints (Variables|Default|GetSpline)) 2))
    (Variables|Default|SetPoints _index)
    (|Wire)))