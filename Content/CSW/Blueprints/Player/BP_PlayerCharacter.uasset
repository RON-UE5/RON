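; BP_PlayerCharacter is the player character Blueprint, adding a night vision toggle on the N key.
; BeginPlay creates a blur animation widget, stores it and adds it to the viewport.
; A FlipFlop on N starts or removes the blur, then after a half-second delay swaps the camera's whole post-process settings between night vision and default presets.
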(event EventBeginPlay
  (bind _returnvalue (UserInterface|CreateWidget "/Game/CSW/Blueprints/HUD/WBP_BlurAnim.WBP_BlurAnim_C"))
  (bind _output_get (Variables|Default|SetBlurAnim _returnvalue))
  (UserInterface|Viewport|AddtoViewport _output_get 0))

(event Collision|EventActorBeginOverlap
  (params (OtherActor :type Actor%20Object%20Reference)))

(event EventTick
  (params (DeltaSeconds :type Float%20%28single-precision%29)))

(event Input|KeyboardEvents|N
  (params (Key :type Key%20Structure :default "None"))
  (bind _bluranim (Variables|Default|GetBlurAnim))
  (bind _cameracomp (Variables|Default|GetCameraComp))
  (:Pressed
    (Utilities|FlowControl|FlipFlop
      (:A
        (UserInterface|Viewport|AddtoViewport _bluranim 0)
        (Default|Start _bluranim)
        (Utilities|FlowControl|Delay 0.5)
        (Variables|/Script/Engine.CameraComponent|SetPostProcessSettings _cameracomp (Variables|Default|GetNightVision%20PP)))
      (:B
        (Default|Remove _bluranim)
        (Utilities|FlowControl|Delay 0.5)
        (Variables|/Script/Engine.CameraComponent|SetPostProcessSettings _cameracomp (Variables|Default|GetDefault%20PP))))))

(fn ConstructionScript)